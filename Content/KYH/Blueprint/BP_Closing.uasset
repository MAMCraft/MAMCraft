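; BP_Closing is an actor Blueprint built to oscillate vertically between two Z limits, though that logic is currently disconnected.
; Up moves it along the actor's up vector and Down along a down vector, both scaled by Speed and delta time without sweep.
; An unreached graph picks between them with the Canup flag and flips it at the height limits.
; Event Tick is empty, so the movement never runs.
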(event `self.ReceiveTick`
  (params (DeltaSeconds :type "Float (single-precision)")))

(fn `down`
  (params (DeltaTime :type "Float (double-precision)"))
  (`self.K2_SetActorLocation` (+ (`self.K2_GetActorLocation`) (* (`self.Speed`) (`KismetMathLibrary.Vector_Down`) DeltaTime))))

(fn `up`
  (params (DeltaTime :type "Float (double-precision)") (NewParam :type "ChildActorComponent Object Reference"))
  (`self.K2_SetActorLocation` (+ (`self.K2_GetActorLocation`) (* DeltaTime (`self.GetActorUpVector`) (`self.Speed`)))))

(fn `UserConstructionScript`)