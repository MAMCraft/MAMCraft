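; Zombie encounter spawner that raises two closing barriers and spawns Num zombie pawns around itself when the player enters Box1.
; Box1 also disables collision on all three boxes, while Box2, if entered earlier, lowers the barriers.
; Each damage event on a spawned zombie, not each death, decrements Num, and reaching zero lowers the barriers.
; Tick slides both barriers between fixed height limits using Canup and Candown flags.
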(event `self.Box1.OnComponentBeginOverlap`
  (params (OverlappedComponent :type "PrimitiveComponent Object Reference") (OtherActor :type "Actor Object Reference") (OtherComp :type "PrimitiveComponent Object Reference") (OtherBodyIndex :type Integer) (bFromSweep :type Boolean) (SweepResult :type "HitResult Structure (by ref)"))
  (cast `/Game/JYS/Blueprints/BP_PlayerCharacter` OtherActor)
  (set `self.canup` true)
  (for _ (range 1 (+ (`self.num`) 1))
    (bind _returnvalue (`|SpawnActorFromClass` "/Game/LSJ/Blueprints/Enermy/BP_ZombiePawn.BP_ZombiePawn_C" (`KismetMathLibrary.MakeTransform` (`KismetMathLibrary.MakeVector` (.x (`KismetMathLibrary.RandomPointInBoundingBox` (`SceneComponent.K2_GetComponentLocation` (`self.DefaultSceneRoot`)) (1000.0 1000.0 0.0))) (.y (`KismetMathLibrary.RandomPointInBoundingBox` (`SceneComponent.K2_GetComponentLocation` (`self.DefaultSceneRoot`)) (1000.0 1000.0 0.0))) (+ (.z (`self.K2_GetActorLocation`)) 100.0))) "AdjustIfPossibleButAlwaysSpawn" "MultiplyWithRoot" null null))
    (add `self.OnTakeAnyDamage` _returnvalue (delegate `CustomEvent`)))
  (`PrimitiveComponent.SetCollisionProfileName` (`self.Box`) "NoCollision" true)
  (`PrimitiveComponent.SetCollisionProfileName` (`self.Box1`) "NoCollision" true)
  (`PrimitiveComponent.SetCollisionProfileName` (`self.Box2`) "NoCollision" true))

(event `CustomEvent` :!signature `self.OnTakeAnyDamage`
  (params (DamagedActor :type "Actor Object Reference") (Damage :type "Float (single-precision)") (DamageType :type "DamageType Object Reference") (InstigatedBy :type "Controller Object Reference") (DamageCauser :type "Actor Object Reference"))
  (bind _output_get (set `self.num` (- (`self.num`) 1)))
  (if (<= _output_get 0)
    (set `self.candown` true)))

(event `self.ReceiveTick`
  (params (DeltaSeconds :type "Float (single-precision)"))
  (bind _bp_closing1 (`self.BP_Closing1`))
  (bind _bp_closing (`self.BP_Closing`))
  (bind _z (.z (`SceneComponent.RelativeLocation` (`self.BP_Closing`))))
  (if (`self.canup`)
    (`self.up` DeltaSeconds _bp_closing1)
    (`self.up` DeltaSeconds _bp_closing)
    (if (>= _z 49.0)
      (set `self.canup` false))
    (elif (`self.candown`)
      (`self.down` DeltaSeconds _bp_closing1)
      (`self.down` DeltaSeconds _bp_closing)
      (if (<= _z -200.0)
        (set `self.candown` false)))))

(event `self.Box2.OnComponentBeginOverlap`
  (params (OverlappedComponent :type "PrimitiveComponent Object Reference") (OtherActor :type "Actor Object Reference") (OtherComp :type "PrimitiveComponent Object Reference") (OtherBodyIndex :type Integer) (bFromSweep :type Boolean) (SweepResult :type "HitResult Structure (by ref)"))
  (cast `/Game/JYS/Blueprints/BP_PlayerCharacter` OtherActor)
  (set `self.candown` true))

(fn `down`
  (params (DeltaTime :type "Float (double-precision)") (NewParam :type "ChildActorComponent Object Reference"))
  (`SceneComponent.K2_SetRelativeLocation` NewParam (+ (`SceneComponent.RelativeLocation` NewParam) (* (`self.Speed`) (`KismetMathLibrary.Vector_Down`) DeltaTime)) false false))

(fn `up`
  (params (DeltaTime :type "Float (double-precision)") (NewParam :type "ChildActorComponent Object Reference"))
  (`SceneComponent.K2_SetRelativeLocation` NewParam (+ (`SceneComponent.RelativeLocation` NewParam) (* DeltaTime (`self.GetActorUpVector`) (`self.Speed`))) false false))

(fn `UserConstructionScript`)